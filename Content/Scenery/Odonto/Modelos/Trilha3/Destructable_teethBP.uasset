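; Destructable tooth Blueprint whose dynamic mesh can be carved or built up at runtime with Geometry Script.
; On BeginPlay it copies a static mesh into the dynamic mesh component, enables complex-as-simple collision and creates a small sphere tool mesh.
; Destruction and Construction events convert the given location to component space, then boolean-subtract or union that sphere.
; A box mesh is also built as SmootherVar, but no graph here uses it.
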(event `/Game/Scenery/BPI_Destruction.Destruction`
  (params (Location :type "Vector Structure"))
  (bind _projectile (`self.Projectile`))
  (`/Engine/EditorBlueprintResources/StandardMacros.IsValid` _projectile
    (:`Is Valid`
      (`GeometryScriptLibrary_MeshBooleanFunctions.ApplyMeshBoolean` (`self.Target Mesh`) (struct) _projectile (`KismetMathLibrary.MakeTransform` (`KismetMathLibrary.InverseTransformLocation` (`SceneComponent.K2_GetComponentToWorld` (`self.DynamicMeshComponent`)) Location)) "Subtract" (struct) null))))

(event `/Game/Scenery/BPI_Construction.Construction`
  (params (Location :type "Vector Structure"))
  (bind _projectile (`self.Projectile`))
  (`/Engine/EditorBlueprintResources/StandardMacros.IsValid` _projectile
    (:`Is Valid`
      (`GeometryScriptLibrary_MeshBooleanFunctions.ApplyMeshBoolean` (`self.Target Mesh`) (struct) _projectile (`KismetMathLibrary.MakeTransform` (`KismetMathLibrary.InverseTransformLocation` (`SceneComponent.K2_GetComponentToWorld` (`self.DynamicMeshComponent`)) Location)) "Union" (struct) null))))

(event `self.ReceiveBeginPlay`
  (`self.BuildMesh`)
  (`|ExecutionSequence`
    (:`then_0`
      (bind _returnvalue (`self.AllocateComputeMesh`))
      (bind _returnvalue_2 (`GeometryScriptLibrary_MeshPrimitiveFunctions.AppendSphereBox` _returnvalue (struct) (struct) 0.8 3 3 3 "Center" null))
      (set `self.Projectile` _returnvalue_2))
    (:`then_1`
      (bind _returnvalue_3 (`self.AllocateComputeMesh`))
      (bind _returnvalue_4 (`GeometryScriptLibrary_MeshPrimitiveFunctions.AppendBox` _returnvalue_3 (struct) (struct) 4.0 4.0 4.0 0 0 0 "Center" null))
      (set `self.SmootherVar` _returnvalue_4))))

(fn `BuildMesh`
  (bind _returnvalue (`BaseDynamicMeshComponent.GetDynamicMesh` (`self.DynamicMeshComponent`)))
  (bind _returnvalue_2 (`DynamicMesh.Reset` _returnvalue))
  (bind _returnvalue_3 (`GeometryScriptLibrary_StaticMeshFunctions.CopyMeshFromStaticMesh` (`self.StaticMesh`) _returnvalue_2 (struct) (struct) null)
    (:`Success`
      (`GeometryScriptLibrary_MeshBasicEditFunctions.AppendMesh` _returnvalue_3 null (struct) false (struct :`CombineMode` "EnableAllMatching") null)
      (`DynamicMeshComponent.EnableComplexAsSimpleCollision` (`self.DynamicMeshComponent`))
      (`KismetSystemLibrary.PrintString` "Hello"))))

(fn `UserConstructionScript`)